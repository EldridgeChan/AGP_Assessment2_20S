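; Procedural map generator that builds a grid of rooms from streaming level instances.
; GenerateMap loops over the grid, instances the level selected by each cell's room type index, then sets it loaded and visible.
; Flattened per-cell arrays supply room type and direction, with transforms placing rooms at fixed spacing and quarter-turn yaw.
; ClearCubes destroys the owner of the actor's static mesh components.
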(event `self.GenerateMap`
  (for _index (range (`self.MapYNum`))
    (for _index_2 (range (`self.MapXNum`))
      (bind _returnvalue (`LevelStreaming.CreateInstance` (`self.StreamingLevels` _index_2 _index) (`KismetStringLibrary.Concat_StrStr` (`KismetStringLibrary.Conv_IntToString` _index) "x" (`KismetStringLibrary.Conv_IntToString` _index_2))))
      (`self.GenerateRoom` (`self.RoomTransform` _index _index_2) _returnvalue))))

(event `self.ClearCubes`
  (for _array_element (`self.K2_GetComponentsByClass` "/Script/Engine.StaticMeshComponent")
    (`self.K2_DestroyActor` (`ActorComponent.GetOwner` _array_element))))

(fn `GenerateRoom`
  (params (RoomTransform :type "Transform Structure") (RoomType :type "LevelStreaming Object Reference"))
  (set `LevelStreaming.LevelTransform` RoomTransform RoomType)
  (set `LevelStreaming.bShouldBeLoaded` true RoomType)
  (set `LevelStreaming.bShouldBeVisible` true RoomType))

(fn `UserConstructionScript`)